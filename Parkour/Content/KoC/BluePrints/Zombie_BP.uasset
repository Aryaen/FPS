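; Zombie Blueprint that repositions itself every tick based on the direction to the player's first-person character.
; BeginPlay caches the player character through a cast.
; Tick scales the normalized zombie-to-player vector to a fixed length and sets it directly as the actor's transform, without adding the current location, sweeping or using delta time.
; Tick also prints an empty string, and the overlap event is unused.
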(event `self.ReceiveBeginPlay`
  ;[1 1 1] Set the Player Variable
  (bind _asfirst_person_character (cast `/Game/FirstPersonBP/Blueprints/FirstPersonCharacter` (`GameplayStatics.GetPlayerCharacter` 0)))
  (set `self.Player` _asfirst_person_character))

(event `self.ReceiveTick`
  (params (DeltaSeconds :type "Float (single-precision)"))
  (`KismetSystemLibrary.PrintText` "")
  (bind _output_get (set `self.Zombie Position` (* (`KismetMathLibrary.Normal` (- (`self.K2_GetActorLocation` (`self.Player`)) (`self.K2_GetActorLocation`))) 100.0)))
  (`self.K2_SetActorTransform` (`KismetMathLibrary.Conv_VectorToTransform` _output_get)))

(fn `UserConstructionScript`)